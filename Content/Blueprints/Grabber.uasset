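; Grabber lets the first-person player pick up Box actors and supplies a location for spawning.
; Both Grab and GetSpawnLocation run a Visibility line trace from player 0's eye viewpoint out to Reach.
; Grab destroys a hit Box and increments the character's Blocks count, up to MaxBlocks.
; GetSpawnLocation returns the impact point on a Box, otherwise the trace end, and draws the trace for debugging.
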(fn `GetReachLineEnd`
  (returns (endPoint :type "Vector Structure"))
  (bind (_outlocation _outrotation) (`Actor.GetActorEyesViewPoint` (`GameplayStatics.GetPlayerCharacter` 0)))
  (return (+ _outlocation (* (`KismetMathLibrary.Conv_RotatorToVector` _outrotation) (`self.Reach`)))))

(fn `GetReachLineStart`
  (returns (LineStart :type "Vector Structure"))
  (return (`Actor.GetActorEyesViewPoint` (`GameplayStatics.GetPlayerCharacter` 0))))

(fn `GetSpawnLocation`
  (returns (SpawnPoint :type "Vector Structure"))
  (bind _linestart (`self.GetReachLineStart`))
  (bind _endpoint (`self.GetReachLineEnd`))
  (bind (_outhit _returnvalue) (`KismetSystemLibrary.LineTraceSingle` :`Start` _linestart :`End` _endpoint :`TraceChannel` "TraceTypeQuery1" :`DrawDebugType` "ForDuration"))
  (if _returnvalue
    (bind (_bblockinghit _binitialoverlap _time _location _impactpoint _normal _impactnormal _physmat _hitactor) (`GameplayStatics.BreakHitResult` _outhit))
    (cast `/Game/Blueprints/Box` _hitactor
      (:`then`
        (return _impactpoint))
      (:`CastFailed`
        _)))
  (return _endpoint))

(fn `Grab`
  (bind _linestart (`self.GetReachLineStart`))
  (bind _endpoint (`self.GetReachLineEnd`))
  (bind _outhit (`KismetSystemLibrary.LineTraceSingle` _linestart _endpoint "TraceTypeQuery1"))
  (bind _asbox (cast `/Game/Blueprints/Box` (`.HitActor` (`GameplayStatics.BreakHitResult` _outhit))))
  (bind _asfirst_person_character (cast `/Game/FirstPersonBP/Blueprints/FirstPersonCharacter` (`GameplayStatics.GetPlayerCharacter` 0)))
  (bind _returnvalue (+ (`/Game/FirstPersonBP/Blueprints/FirstPersonCharacter.Blocks` _asfirst_person_character) 1))
  (`/Engine/EditorBlueprintResources/StandardMacros.CompareInt` _returnvalue (`/Game/FirstPersonBP/Blueprints/FirstPersonCharacter.MaxBlocks` _asfirst_person_character)
    (:`==`
      _)
    (:`<`
      _))
  (set `/Game/FirstPersonBP/Blueprints/FirstPersonCharacter.Blocks` _returnvalue _asfirst_person_character)
  (`Actor.K2_DestroyActor` _asbox))